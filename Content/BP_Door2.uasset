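; BP_Door2 is a door actor that opens once enough buttons are pressed and triggers level streaming.
; Each tick it compares the first-person game mode's button counter to its ButtonQuantity, then disables collision, hides the cube and loads the streaming level.
; ActivateDoor2 reverses the opening by restoring collision, showing the cube and printing a debug message.
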(event Custom|ActivateDoor2
  (Collision|SetActorEnableCollision true)
  (Development|SetHiddeninGame (Variables|Default|GetCube) false false)
  (Development|PrintString "activated"))

(event EventTick
  (params (DeltaSeconds :type Float%20%28single-precision%29))
  (bind _asbp_first_person_game_mode (Utilities|Casting|CastToBP_FirstPersonGameMode (Game|GetGameMode)))
  (if (== (Variables|/Game/FirstPerson/Blueprints/BP_FirstPersonGameMode.BP_FirstPersonGameMode_C|GetCounterButton _asbp_first_person_game_mode) (Variables|Default|GetButtonQuantity))
    (Collision|SetActorEnableCollision false)
    (Development|SetHiddeninGame (Variables|Default|GetCube) true false)
    (Class|GameplayStatics|LoadStreamLevelbySoftObjectPtr "/Game/FirstPerson/LVL_Streaming.LVL_Streaming" true false)))

(fn ConstructionScript)