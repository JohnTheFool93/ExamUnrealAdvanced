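; Elevator actor that moves its Cube up and down once the BP_FirstPersonGameMode Counter equals TriggerQuantity.
; Tick polls the counter and plays or reverses the ElevatorUpdown timeline based on IsRising, which flips whenever the timeline finishes.
; The track drives relative Z from zero, while X and Y reuse the world location captured at BeginPlay.
; Destination is computed at BeginPlay but never read.
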(event EventBeginPlay
  (bind _output_get (Variables|Default|SetStart (Transformation|GetWorldLocation (Variables|Default|GetCube))))
  (Variables|Default|SetDestination (+ _output_get "0.000000,0.000000,1000.000000")))

(event EventTick
  (params (DeltaSeconds :type Float%20%28single-precision%29))
  (bind _start (Variables|Default|GetStart))
  (bind (_x _y) (Math|Vector|BreakVector _start))
  (bind _asbp_first_person_game_mode (Utilities|Casting|CastToBP_FirstPersonGameMode (Game|GetGameMode)))
  (if (== (Variables|/Game/FirstPerson/Blueprints/BP_FirstPersonGameMode.BP_FirstPersonGameMode_C|GetCounter _asbp_first_person_game_mode) (Variables|Default|GetTriggerQuantity))
    (if (Variables|Default|GetIsRising)
      (bind _elevatortrack (Timeline|Elevator%20up/down Play)
        (:Update
          (Transformation|SetRelativeLocation (Variables|Default|GetCube) (Math|Vector|MakeVector _x _y (* _elevatortrack 1e+03)) false false))
        (:Finished
          (Variables|Default|SetIsRising (not (Variables|Default|GetIsRising)))))
      (else
        (Timeline|Elevator%20up/down Reverse)))))

(fn ConstructionScript)